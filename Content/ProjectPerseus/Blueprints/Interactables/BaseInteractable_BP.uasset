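; Base interactable pickup actor that gives its item to the top-down player character.
; The construction script fills ItemInfo from the ItemInfo data table, using the ItemName enum converted to a row name.
; BeginPlay caches the player as BP_TopDownCharacter.
; Interact passes ItemInfo to the player's PickupItem, then destroys the actor.
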(event `self.ReceiveBeginPlay`
  (bind _asbp_top_down_character (cast `/Game/TopDown/Blueprints/BP_TopDownCharacter` (`GameplayStatics.GetPlayerCharacter` 0)))
  (set `self.Player` _asbp_top_down_character))

(event `/Game/ProjectPerseus/Data/InteractBPI.Interact`
  (`/Game/TopDown/Blueprints/BP_TopDownCharacter.PickupItem` (`self.Player`) (`self.ItemInfo`))
  (`self.K2_DestroyActor`))

(fn `UserConstructionScript`
  (bind _returnvalue (`|GetDataTableRow` "/Game/ProjectPerseus/Data/ItemInfo_DT.ItemInfo_DT" (`KismetStringLibrary.Conv_StringToName` (`|GetEnumeratorNameAsString` (`self.ItemName`))))
    (:`then`
      (set `self.ItemInfo` _returnvalue))))